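; Behavior tree task that starts a dialogue in the DialogueTree by showing the dialogue UI.
; On execute, it gets the dialogue widget from the HUD reference in BP_Game_Mode_PCC and makes it visible.
; It stores that widget in a blackboard key for later line display, disables player character input and finishes successfully.
; An unused pawn-based variant and mouse-cursor nodes remain disconnected.
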(event EventReceiveExecuteAI
  (params (OwnerController :type AI%20Controller%20Object%20Reference) (ControlledPawn :type Pawn%20Object%20Reference))
  ;[0.7011 1 0.6924] Character
  ;;[1 1 1] PAWN Gets Widget_dialogue var in BP Game mode and changes visiblity
  (bind _asbp_game_mode_pcc (Utilities|Casting|CastToBP_Game_Mode_PCC (Game|GetGameMode)))
  (Widget|SetVisibility (Variables|/Game/Dialogue/Widget/HUD_Dialogue.HUD_Dialogue_C|GetWidget_Dialogue (Variables|/Game/Dialogue/BluePrints/Player/BP_Game_Mode_PCC.BP_Game_Mode_PCC_C|GetHUDDialogueInBPGameModePCC _asbp_game_mode_pcc)) "Visible")
  ;;[1 1 1] Stores temp value in "BB_Dialogue_UI in Start Dia" as same state/value as "Widget_dialogue", which is then stored in blackboard
  ;;
  ;; Sets BB value as object, which dialogue box being displayed
  ;;
  ;; Note: links to DialogueWidgetInDisplayLine
  (Class|BTFunctionLibrary|SetBlackboardValueasObject (Variables|Default|GetBB_Dialogue_UIInStartDialogue) (Variables|/Game/Dialogue/Widget/HUD_Dialogue.HUD_Dialogue_C|GetWidget_Dialogue (Variables|/Game/Dialogue/BluePrints/Player/BP_Game_Mode_PCC.BP_Game_Mode_PCC_C|GetHUDDialogueInBPGameModePCC _asbp_game_mode_pcc)))
  (Input|DisableInput (Game|GetPlayerCharacter 0) (Game|GetPlayerController 0))
  (AI|BehaviorTree|FinishExecute true))