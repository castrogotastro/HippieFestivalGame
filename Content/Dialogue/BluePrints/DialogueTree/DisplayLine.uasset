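; Behavior tree task that displays one line of dialogue in the dialogue tree.
; On execute it gets the Widget_Dialogue from the blackboard and sets its dialogue text to the task's TextDisplay.
; Tick checks the InteractClose action's mapped keys to finish the task as failed, but only behind an outer key-press check whose key is None.
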(event EventReceiveExecuteAI
  (params (OwnerController :type AI%20Controller%20Object%20Reference) (ControlledPawn :type Pawn%20Object%20Reference))
  ;[1 1 1] Get Blackboard Value as Object is generic. Therefore, must cast to Widget_Dialogue to define
  ;;[1 1 1] Tells Var "Dialogue Widget in Display Line" to show text in Widget Dialgoue. Text can be defined here with var "Text Display"
  (bind _aswidget_dialogue (Utilities|Casting|CastToWidget_Dialogue (Class|BTFunctionLibrary|GetBlackboardValueasObject (Variables|Default|GetDialogueWidgetInDisplayLine))))
  ;[1 1 1] Set var "Dialogue Text" in Widget_Dialogue to var "Text Display"
  (Variables|/Game/Dialogue/Widget/Widget_Dialogue.Widget_Dialogue_C|SetDialogueText _aswidget_dialogue (Variables|Default|GetTextDisplay)))

(event EventTick
  (params (OwnerActor :type Actor%20Object%20Reference) (DeltaSeconds :type Float%20%28single-precision%29))
  ;[1 0.3811 0.4509] Checks if player pressed specified key that ends dialogue. Change to button at end of dialogue
  (if (Game|Player|WasInputKeyJustPressed (Game|GetPlayerController 0) "None")
    ;;[1 1 1] Loops/cycles through all keys with interaction name in project settings
    (for _array_element (Class|InputSettings|GetActionMappingbyName (Class|InputSettings|GetInputSettings) "InteractClose")
      (if (Game|Player|WasInputKeyJustPressed (Game|GetPlayerController 0) (.Key (Utilities|Struct|BreakInputActionKeyMapping _array_element)))
        (AI|BehaviorTree|FinishExecute false)))))