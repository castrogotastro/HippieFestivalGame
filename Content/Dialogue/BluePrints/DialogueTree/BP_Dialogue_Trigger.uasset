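; Dialogue trigger actor that opens a HUD_DialogueWASD widget for the first player when interacted with or clicked.
; Clicking toggles the stored widget by removing or recreating it, while OnInteract always creates a new one without checking.
; No live path calls AddToViewport; disconnected leftovers show an older Widget_DialogueWASD version that did, and passed in dialogue text.
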(event EventBeginPlay)

(event Collision|EventActorBeginOverlap
  (params (OtherActor :type Actor%20Object%20Reference)))

(event EventTick
  (params (DeltaSeconds :type Float%20%28single-precision%29)))

(event EventOnInteract
  (params (MouseInteractor :type Mouse%20Cursor%20Interactor%20Object%20Reference))
  (bind _returnvalue (UserInterface|CreateWidget "/Game/Dialogue/BluePrints/DialogueTree/Widget/WidgetsWASD/HUD_DialogueWASD.HUD_DialogueWASD_C" (Game|GetPlayerController 0)))
  (Variables|Default|SetPlayerHUDInBPTrigger _returnvalue))

(event MouseInput|EventActorOnClicked
  (params (ButtonPressed :type Key%20Structure :default "None"))
  ;[1 1 1] Open dialogue box when actor clicked
  ;;[1 1 1] Checks if dialogue box already open. If Actor clicked again, dialogue box closes
  (Utilities|IsValid (Variables|Default|GetPlayerHUDInBPTrigger)
    (:Is%20Valid
      (Widget|RemovefromParent (Variables|Default|GetPlayerHUDInBPTrigger))
      (Variables|Default|SetPlayerHUDInBPTrigger 0))
    (:Is%20Not%20Valid
      (bind _returnvalue (UserInterface|CreateWidget "/Game/Dialogue/BluePrints/DialogueTree/Widget/WidgetsWASD/HUD_DialogueWASD.HUD_DialogueWASD_C" (Game|GetPlayerController 0)))
      (Variables|Default|SetPlayerHUDInBPTrigger _returnvalue))))

(fn ConstructionScript)