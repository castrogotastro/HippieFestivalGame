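; NPC Blueprint that starts a dialogue when the player interacts with it.
; On BeginPlay it copies its DialogueTreeInNPC behaviour tree, meant to be chosen per instance, into its NPC_AI_Behaviour_Tree AI controller.
; OnInteract casts to that controller and calls StartDialogue.
; The Construction Script repeats the tree assignment, though its note says the controller is inaccessible there, hence the BeginPlay copy.
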(event Collision|EventActorBeginOverlap
  (params (OtherActor :type Actor%20Object%20Reference)))

(event EventTick
  (params (DeltaSeconds :type Float%20%28single-precision%29)))

(event EventOnInteract
  (params (MouseInteractor :type Mouse%20Cursor%20Interactor%20Object%20Reference))
  ;[1 1 1] On Interatct Event (Mouse click on NPC) the Start Dialogue Custom Event within NPC_AI_Behaviour is trigger
  (bind _asnpc_ai_behaviour_tree (Utilities|Casting|CastToNPC_AI_Behaviour_Tree (AI|GetAIController self)))
  (Default|StartDialogue _asnpc_ai_behaviour_tree))

(event EventBeginPlay
  ;[1 1 1] Makes Behaviour Tree drop down visible on details window when NPC is selected in viewport
  (bind _asnpc_ai_behaviour_tree (Utilities|Casting|CastToNPC_AI_Behaviour_Tree (AI|GetAIController self)))
  (Variables|/Game/Dialogue/BluePrints/NPC/NPC_AI_Behaviour_Tree.NPC_AI_Behaviour_Tree_C|SetDialogueTreeInNPC_AIBehaviour _asnpc_ai_behaviour_tree (Variables|Default|GetDialogueTreeInNPC)))

(fn ConstructionScript
  ;[1 1 1] Makes Behaviour Tree drop down visible on details window when NPC is selected in viewport
  ;
  ; NOTE: AI_Controler isn't accessible through Construction Script; thereofre, this blueprint was moved to Event Graph
  (bind _asnpc_ai_behaviour_tree (Utilities|Casting|CastToNPC_AI_Behaviour_Tree (AI|GetAIController self)))
  (Variables|/Game/Dialogue/BluePrints/NPC/NPC_AI_Behaviour_Tree.NPC_AI_Behaviour_Tree_C|SetDialogueTreeInNPC_AIBehaviour _asnpc_ai_behaviour_tree (Variables|Default|GetDialogueTreeInNPC)))