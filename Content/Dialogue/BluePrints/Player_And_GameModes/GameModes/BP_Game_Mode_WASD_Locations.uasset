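; Game mode for the WASD location levels that runs a festival countdown and day/night clock.
; BeginPlay loads time and rotation from GameInstance_WASD, creates the dialogue HUD and sets player input, locking mouse look.
; A Tick delay counts down, syncing to the GameInstance via dispatchers; each minute (one game hour) adjusts energy, anxiety, sky rotation and time-based NPCs.
; At zero it shows StartMenu and pauses the game.
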(event Custom|UpdateTimer_Event
  (params (minutes :type Integer) (seconds :type Integer))
  (bind _as_game_instance_wasd_ref (Variables|Default|GetAs%20Game%20Instance%20WASD%20ref))
  ;[1 1 1] Comment
  ;;[1 1 1] Cast to GameInstant and promote to Var to use above.
  ;;
  ;; Init Timer: Set Seconds and Minutes varialber in this BP to those in GameInstance when BeginPlay fires.
  ;;;[1 1 1] Sec & min var in EventDispatch node are those in THIS BP
  ;;;[1 1 1] Set Sec & Min Var in GameInst to those in this BP
  (bind _output_get (Variables|/Game/Dialogue/BluePrints/Game_Instance/GameInstance_WASD.GameInstance_WASD_C|SetINT_MInutes _as_game_instance_wasd_ref minutes))
  (bind _output_get_2 (Variables|/Game/Dialogue/BluePrints/Game_Instance/GameInstance_WASD.GameInstance_WASD_C|SetINT_Seconds _as_game_instance_wasd_ref seconds))
  (Variables|Default|SetMinutes_ConvertedtoHours _output_get)
  (Variables|Default|SetSeconds_convertedtoMinutes _output_get_2))

(event Custom|UpdateTimerMinutestoHoursClock_Event
  (params (Rotation :type Float%20%28single-precision%29))
  ;[1 1 1] Comment
  (bind _output_get (Variables|/Game/Dialogue/BluePrints/Game_Instance/GameInstance_WASD.GameInstance_WASD_C|SetINT_RotationDayNightCycle (Variables|Default|GetAs%20Game%20Instance%20WASD%20ref) Rotation))
  (Variables|Default|SetRotation _output_get))

(event EventAnimateinOutWidgetBoxes
  (params (SlideInIfTrue :type Boolean) (NPC_InteractMessage_Ref :type NPC%20Interact%20Message%20PCC%20Object%20Reference) (Widget_DialogueWASD_Ref :type Widget%20Dialogue%20WASD%20Object%20Reference) (MainMap :type Main%20Map%20Click%20to%20Load%20Object%20Reference))
  ;[1 0.1172 0] Unused Animation
  (if SlideInIfTrue
    (bind _lerp (Timeline|Timeline_1 PlayFromStart)
      (:Update
        (Variables|Default|SetX_Axis_PositionInteractMessage (+ (* _lerp (- (Variables|Default|GetStartPositionInteractMessage) (Variables|Default|GetEndPositionInteractMessage))) (Variables|Default|GetStartPositionInteractMessage)))))
    (else
      (Timeline|Timeline_1 ReverseFromEnd))))

(event EventTick
  (params (DeltaSeconds :type Float%20%28single-precision%29))
  (bind _pcccharacter_sprite_locations (Variables|Default|GetPCCCharacter%20Sprite%20Locations))
  ;[1 1 1] Timer
  (Utilities|FlowControl|Delay 0.1)
  (if (== (Variables|Default|GetSeconds_convertedtoMinutes) 0)
    (if (== (Variables|Default|GetMinutes_ConvertedtoHours) 0)
      ;;[1 1 1] Game over when timer = 0
      (bind _returnvalue (UserInterface|CreateWidget "/Game/Dialogue/BluePrints/MainMenu_Widget/StartMenu.StartMenu_C"))
      (UserInterface|Viewport|AddtoViewport _returnvalue 0)
      (Game|SetGamePaused true)
      (else
        ;;[1 1 1] Sets timer to new minute and 59 sec.
        ;;
        ;; Updates sec & min var in GameInstance
        (bind _output_get (Variables|Default|SetSeconds_convertedtoMinutes 59))
        (bind _output_get_2 (Variables|Default|SetMinutes_ConvertedtoHours (- (Variables|Default|GetMinutes_ConvertedtoHours) 1)))
        (Default|CallUpdateTimerMinutesSecondstoHoursMinutesTimeRemaining _output_get_2 _output_get)
        ;;[1 1 1] Update Progress bar based on time
        (Default|EnergyDecreaseFunction _pcccharacter_sprite_locations 0.1)
        (Default|AnxietyIncreaseFunction _pcccharacter_sprite_locations 0.1)
        (Utilities|FlowControl|Sequence
          (:then_0
            ;[1 1 1] Timer for Day and Night Cycle. And Tiem of day hours
            ;;[1 1 1] If hours left at festival are less-than or = to 12, then TimeOfDay_hours equals HoursLeftAtFestival + 12 so festival ends at 12:00pm (noon)
            ;;
            ;; Starts at Day 0
            (if (and (>= (Variables|Default|GetMinutes_ConvertedtoHours) 0) (<= (Variables|Default|GetMinutes_ConvertedtoHours) 12))
              (Variables|Default|SetTimeOfDay_Hours_24hrclock (- 12 (Variables|Default|GetMinutes_ConvertedtoHours)))
              ;;[1 1 1] Calc Rotation
              (if (== (Variables|Default|GetMinutes_ConvertedtoHours) 0)
                (bind _output_get_3 (Variables|Default|SetRotation -89.0))
                (Default|CallUpdateTimerMinutestoHoursClock _output_get_3)
                (elif (and (>= (Variables|Default|GetMinutes_ConvertedtoHours) 1) (<= (Variables|Default|GetMinutes_ConvertedtoHours) 12))
                  (bind _output_get_4 (Variables|Default|SetRotation (+ -89.0 (* 14.0 (Math|Conversions|ToFloat(Integer) (Variables|Default|GetMinutes_ConvertedtoHours))))))))))
          (:then_1
            ;;[1 1 1] If hours left at festival are less-than or = to 12, then TimeOfDay_hours equals HoursLeftAtFestival
            ;;
            ;; 11:00pm(23:00) Day1
            ;; to
            ;; 12:00am (0:00) Day 1
            (if (and (<= (Variables|Default|GetMinutes_ConvertedtoHours) 36) (>= (Variables|Default|GetMinutes_ConvertedtoHours) 13))
              (Variables|Default|SetTimeOfDay_Hours_24hrclock (- (+ 24 12) (Variables|Default|GetMinutes_ConvertedtoHours)))
              ;;[1 1 1] Calc Rotation
              (if (and (>= (Variables|Default|GetMinutes_ConvertedtoHours) 13) (<= (Variables|Default|GetMinutes_ConvertedtoHours) 24))
                (bind _output_get_5 (Variables|Default|SetRotation (- 89.0 (* 14.0 (- (Math|Conversions|ToFloat(Integer) (Variables|Default|GetMinutes_ConvertedtoHours)) 12.0)))))
                (Default|CallUpdateTimerMinutestoHoursClock _output_get_5)
                (elif (and (>= (Variables|Default|GetMinutes_ConvertedtoHours) 25) (<= (Variables|Default|GetMinutes_ConvertedtoHours) 36))
                  (bind _output_get_6 (Variables|Default|SetRotation (+ -89.0 (* 14.0 (- (Math|Conversions|ToFloat(Integer) (Variables|Default|GetMinutes_ConvertedtoHours)) 24.0)))))
                  (Default|CallUpdateTimerMinutestoHoursClock _output_get_6)))))
          (:then_2
            ;;[1 1 1] If hours left at festival are less-than or = to 12, then TimeOfDay_hours equals HoursLeftAtFestival
            ;;
            ;; Day 2 (12:00pm noon) to Day 3 (12:00pm midnight)
            (if (and (<= (Variables|Default|GetMinutes_ConvertedtoHours) 49) (>= (Variables|Default|GetMinutes_ConvertedtoHours) 37))
              (Variables|Default|SetTimeOfDay_Hours_24hrclock (- (+ 48 12) (Variables|Default|GetMinutes_ConvertedtoHours)))
              ;;[1 1 1] Calc Rotation
              (if (and (>= (Variables|Default|GetMinutes_ConvertedtoHours) 37) (<= (Variables|Default|GetMinutes_ConvertedtoHours) 48))
                (bind _output_get_7 (Variables|Default|SetRotation (- 89.0 (* 14.0 (- (Math|Conversions|ToFloat(Integer) (Variables|Default|GetMinutes_ConvertedtoHours)) 36.0)))))
                (Default|CallUpdateTimerMinutestoHoursClock _output_get_7)
                (elif (and (>= (Variables|Default|GetMinutes_ConvertedtoHours) 49) (<= (Variables|Default|GetMinutes_ConvertedtoHours) 52))
                  (bind _output_get_8 (Variables|Default|SetRotation -79.0))
                  (Default|CallUpdateTimerMinutestoHoursClock _output_get_8)))))
          (:then_3
            (bind _outactors (Actor|GetAllActorsOfClass "/Game/Dialogue/BluePrints/NPC/WASD_NPC/NPC_WASDTesh.NPC_WASDTesh_C"))
            (Default|ShowNPCTeshTimeBased (Utilities|Array|Get(acopy) _outactors))
            (bind _outactors_2 (Actor|GetAllActorsOfClass "/Game/Dialogue/BluePrints/NPC/WASD_NPC/NPC_WASD.NPC_WASD_C"))
            (Default|ShowNPCNPCBaseTimeBased (Utilities|Array|Get(acopy) _outactors_2))))))
    (else
      ;;[1 1 1] If seconds>0 then update seconds to Seconds - 1
      ;;
      ;; Update Seconds var in GameInstance
      (bind _output_get_9 (Variables|Default|SetSeconds_convertedtoMinutes (- (Variables|Default|GetSeconds_convertedtoMinutes) 1)))
      (Default|CallUpdateTimerMinutesSecondstoHoursMinutesTimeRemaining (Variables|Default|GetMinutes_ConvertedtoHours) _output_get_9))))

(event EventBeginPlay
  ;[1 1 1] Comment
  ;;[1 1 1] Cast to GameInstant and promote to Var to use above.
  ;;
  ;; Init Timer: Set Seconds and Minutes varialber in this BP to those in GameInstance when BeginPlay fires.
  (bind _asgame_instance_wasd (Utilities|Casting|CastToGameInstance_WASD (Game|GetGameInstance)))
  (Variables|Default|SetAs%20Game%20Instance%20WASD%20ref _asgame_instance_wasd)
  (EventDispatchers|BindEventtoUpdateTimerMinutesSecondstoHoursMinutesTimeRemaining (delegate Custom|UpdateTimer_Event))
  ;;;[1 1 1] Pulls sec & min var from GameInst & sets sec & min var on THIS BP when BeginPlay fires
  (Variables|Default|SetMinutes_ConvertedtoHours (stale Custom|UpdateTimer_Event _output_get))
  (Variables|Default|SetSeconds_convertedtoMinutes (stale Custom|UpdateTimer_Event _output_get_2))
  (EventDispatchers|BindEventtoUpdateTimerMinutestoHoursClock (delegate Custom|UpdateTimerMinutestoHoursClock_Event))
  (Variables|Default|SetRotation (stale Custom|UpdateTimerMinutestoHoursClock_Event _output_get))
  ;;[1 1 1] Initial dialogue text when game play begins
  ;;;[0 1 0.3069] Add HUD to viewport - Toggle widgets on and off using this ref
  (bind _returnvalue (UserInterface|CreateWidget "/Game/Dialogue/BluePrints/DialogueTree/Widget/WidgetsWASD/HUD_DialogueWASD.HUD_DialogueWASD_C"))
  (bind _output_get (Variables|Default|SetHeadsUpDisplay_Dialogue_WASD _returnvalue))
  (UserInterface|Viewport|AddtoViewport _output_get 0)
  (bind _aspcccharacter_sprite_locations (Utilities|Casting|CastToPCCCharacterSprite_Locations (Game|GetPlayerCharacter 0)))
  (bind _output_get_2 (Variables|Default|SetPCCCharacter%20Sprite%20Locations _aspcccharacter_sprite_locations))
  (Variables|Default|SetDisableInputAtStartInBPGameMode true)
  (if (Variables|Default|GetDisableInputAtStartInBPGameMode)
    (Variables|Default|SetEnableMouseButNoMovement true)
    (if (Variables|Default|GetEnableMouseButNoMovement)
      (Utilities|FlowControl|Sequence
        (:then_0
          ;;;[1 1 1] Set both "DisableWASDEnableMouseClickOnly" and "DisableMouseLookEnableMouseClickOnly" to TRUE to
          ;;;
          ;;; disable player WASD movement and disable player looking around with mouse, but Enable mouse to click and move in environment
          ;;;;[1 1 1] Set Var "DisableInputAtStartInBP" to TRUE and "EnableMouseButton" to FALSE and "DisableWASDEnableMouseClickOnly" to TRUE to:
          ;;;;
          ;;;; Enable Mouse movement, but disable Player movement with WASD
          (Variables|Default|SetDisableWASDEnableMouseClickOnly false)
          (Input|SetIgnoreMoveInput (Game|GetPlayerController 0) (Variables|Default|GetDisableWASDEnableMouseClickOnly)))
        (:then_1
          ;;;;[1 1 1] Set Var "DisableInputAtStartInBP" to TRUE and "EnableMouseButton" to FALSE and "DisableMouseLookEnableMouseClickOnly" to TRUE to:
          ;;;;
          ;;;; Enable Mouse movement, but disable Player looking around with mouse
          (Variables|Default|SetDisableMouseLookEnableMouseClickOnly true)
          (Input|SetIgnoreLookInput (Game|GetPlayerController 0) (Variables|Default|GetDisableMouseLookEnableMouseClickOnly))))
      (else
        ;;;[1 1 1] Set Var "DisableInputAtStartInBP" to TRUE and "EnableMouseButton" to FALSE to:
        ;;;
        ;;; Disable ALL player input
        (Input|DisableInput (Game|GetPlayerCharacter 0) (Game|GetPlayerController 0))))
    (else
      ;;;[1 1 1] Set Var "DisableInputAtStartInBP" to False to Enable ALL player input
      (Input|EnableInput (Game|GetPlayerCharacter 0) (Game|GetPlayerController 0)))))

(event Input|ActionEvents|InputActionTest
  (params (Key :type Key%20Structure :default "None"))
  ;[1 1 1] Comment
)

(fn ConstructionScript)