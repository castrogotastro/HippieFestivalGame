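; Game mode for the PCC Locations levels that runs a countdown clock and ends the game when time runs out.
; BeginPlay adds the dialogue HUD, caches the player sprite character, and uses hardcoded flags to allow movement but ignore look input.
; A one-second Delay on Tick drives the clock, lowering energy and raising anxiety at each minute rollover.
; At zero it shows the Game Over widget and pauses.
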(event EventTick
  (params (DeltaSeconds :type Float%20%28single-precision%29))
  (bind _pcccharacter_sprite_locations (Variables|Default|GetPCCCharacter%20Sprite%20Locations))
  (Utilities|FlowControl|Delay 1.0)
  (if (== (Variables|Default|GetSeconds) 0)
    (if (== (Variables|Default|GetMinutes) 0)
      (bind _returnvalue (UserInterface|CreateWidget "/Game/Dialogue/BluePrints/MainMenu_Widget/Game_Over.Game_Over_C"))
      (UserInterface|Viewport|AddtoViewport _returnvalue 0)
      (Game|SetGamePaused true)
      (else
        (Variables|Default|SetSeconds 59)
        (Default|EnergyDecreaseFunction _pcccharacter_sprite_locations 0.2)
        (Default|AnxietyIncreaseFunction _pcccharacter_sprite_locations 0.2)
        (Variables|Default|SetMinutes (- (Variables|Default|GetMinutes) 1))))
    (else
      (Variables|Default|SetSeconds (- (Variables|Default|GetSeconds) 1)))))

(event EventBeginPlay
  ;[1 1 1] Set Game Mode
  (Input|SetInputModeGameOnly (Game|GetPlayerController 0))
  ;[1 1 1] Initial dialogue text when game play begins
  ;;[1 1 1] Add HUD to viewport
  (bind _returnvalue (UserInterface|CreateWidget "/Game/Dialogue/BluePrints/DialogueTree/Widget/HUD_Dialogue.HUD_Dialogue_C"))
  (bind _output_get (Variables|Default|SetHeadsUpDisplay_Dialogue_WASD _returnvalue))
  (UserInterface|Viewport|AddtoViewport _output_get 0)
  (bind _aspcccharacter_sprite_locations (Utilities|Casting|CastToPCCCharacterSprite_Locations (Game|GetPlayerCharacter 0)))
  (Variables|Default|SetPCCCharacter%20Sprite%20Locations _aspcccharacter_sprite_locations)
  (Variables|Default|SetDisableInputAtStartInBPGameMode true)
  (if (Variables|Default|GetDisableInputAtStartInBPGameMode)
    (Variables|Default|SetEnableMouseButNoMovement true)
    (if (Variables|Default|GetEnableMouseButNoMovement)
      (Utilities|FlowControl|Sequence
        (:then_0
          ;;[1 1 1] Set both "DisableWASDEnableMouseClickOnly" and "DisableMouseLookEnableMouseClickOnly" to TRUE to
          ;;
          ;; disable player WASD movement and disable player looking around with mouse, but Enable mouse to click and move in environment
          ;;;[1 1 1] Set Var "DisableInputAtStartInBP" to TRUE and "EnableMouseButton" to FALSE and "DisableWASDEnableMouseClickOnly" to TRUE to:
          ;;;
          ;;; Enable Mouse movement, but disable Player movement with WASD
          (Variables|Default|SetDisableWASDEnableMouseClickOnly false)
          (Input|SetIgnoreMoveInput (Game|GetPlayerController 0) (Variables|Default|GetDisableWASDEnableMouseClickOnly)))
        (:then_1
          ;;;[1 1 1] Set Var "DisableInputAtStartInBP" to TRUE and "EnableMouseButton" to FALSE and "DisableMouseLookEnableMouseClickOnly" to TRUE to:
          ;;;
          ;;; Enable Mouse movement, but disable Player looking around with mouse
          (Variables|Default|SetDisableMouseLookEnableMouseClickOnly true)
          (Input|SetIgnoreLookInput (Game|GetPlayerController 0) (Variables|Default|GetDisableMouseLookEnableMouseClickOnly))))
      (else
        ;;[1 1 1] Set Var "DisableInputAtStartInBP" to TRUE and "EnableMouseButton" to FALSE to:
        ;;
        ;; Disable ALL player input
        (Input|DisableInput (Game|GetPlayerCharacter 0) (Game|GetPlayerController 0))))
    (else
      ;;[1 1 1] Set Var "DisableInputAtStartInBP" to False to Enable ALL player input
      (Input|EnableInput (Game|GetPlayerCharacter 0) (Game|GetPlayerController 0)))))

(fn ConstructionScript)