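; Default pawn for mouse-driven interaction, which enables the cursor, click and hover events and takes the dialogue HUD from BP_Game_Mode_Change_Pawn.
; Tick and Interact call InteractCheck, with Interact sending OnInteractMessage to its result.
; InteractCheck's cursor trace for BP_Interaction_Interface physics bodies, which toggles the HUD message, is disconnected, so the function does nothing.
; Left click is test code printing the pawn under the cursor.
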(event Collision|EventActorBeginOverlap
  (params (OtherActor :type Actor%20Object%20Reference))
  ;[1 1 1] Test code for interactions occuring when mouse hovers over a slected object type
)

(event EventBeginPlay
  (bind _returnvalue (Game|GetPlayerController 0))
  ;[1 1 1] Enable Mouse Click and Hover & Show Mouse Cursor
  (Variables|/Script/Engine.PlayerController|SetbEnableClickEvents _returnvalue true)
  (Variables|/Script/Engine.PlayerController|SetbEnableMouseOverEvents _returnvalue true)
  (Variables|/Script/Engine.PlayerController|SetbShowMouseCursor _returnvalue true)
  ;[1 1 1] Text display in Game Mode. Makes Var from HUDDialogueInBPGameMode with name "PlayerHUDInBPDefaultPawn"
  (bind _asbp_game_mode_change_pawn (Utilities|Casting|CastToBP_Game_Mode_Change_Pawn (Game|GetGameMode)))
  (Variables|Default|SetPlayerHUDInBPDefaultPawn (Variables|/Game/Dialogue/BluePrints/Player_And_GameModes/GameModes/BP_Game_Mode_Change_Pawn.BP_Game_Mode_Change_Pawn_C|GetHUDDialogueInBPGameMode _asbp_game_mode_change_pawn)))

(event EventTick
  (params (DeltaSeconds :type Float%20%28single-precision%29))
  ;[1 0 0.01685] Copy to Character
  (CallFunction|InteractCheck))

(event Input|ActionEvents|InputActionInteract
  (params (Key :type Key%20Structure))
  ;[1 0 0.01685] Copy to Character
  (:Pressed
    (bind _actorcheck (CallFunction|InteractCheck))
    (Class|BPInteractionInterface|OnInteract(Message) _actorcheck)))

(event Input|MouseEvents|LeftMouseButton
  (params (Key :type Key%20Structure))
  (bind _returnvalue (Game|GetPlayerController 0))
  ;[1 1 1] Test code for interactions occuring when mouse hovers over a slected object type
  (:Pressed
    (if (.ReturnValue (Game|Player|GetHitResultUnderCursorbyChannel _returnvalue "TraceTypeQuery1" true))
      (Development|PrintString (Utilities|GetDisplayName (.HitActor (Collision|BreakHitResult (.HitResult (Class|PlayerController|GetHitResultUnderCursorforObjects _returnvalue (Utilities|Array|MakeArray "ObjectTypeQuery3") true)))))))))

(fn ConstructionScript)

(fn InteractCheck)