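; Game mode Blueprint for the old-version mouse-and-pawn player setup that shows dialogue and configures player input when play begins.
; BeginPlay sets game-only input, then creates, stores and adds the dialogue HUD widget to the viewport.
; Hard-set boolean toggles choose between full, partial or disabled input.
; As set, move input stays active despite the "NoMovement" flag name, while look input is ignored.
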(event EventTick
  (params (DeltaSeconds :type Float%20%28single-precision%29)))

(event EventBeginPlay
  (Input|SetInputModeGameOnly (Game|GetPlayerController 0))
  ;[1 1 1] Initial dialogue text when game play begins
  (bind _returnvalue (UserInterface|CreateWidget "/Game/Dialogue/BluePrints/DialogueTree/Widget/OLD_Widgets/HUD_DialogueBPRef.HUD_DialogueBPRef_C"))
  (bind _output_get (Variables|Default|SetHUDDialogueInBPGameModePCC _returnvalue))
  (UserInterface|Viewport|AddtoViewport _output_get 0)
  (Variables|Default|SetDisableInputAtStartInBPGameMode true)
  (if (Variables|Default|GetDisableInputAtStartInBPGameMode)
    (Variables|Default|SetEnableMouseButNoMovement true)
    (if (Variables|Default|GetEnableMouseButNoMovement)
      (Utilities|FlowControl|Sequence
        (:then_0
          ;;[1 1 1] Set both "DisableWASDEnableMouseClickOnly" and "DisableMouseLookEnableMouseClickOnly" to TRUE to
          ;;
          ;; disable player WASD movement and disable player looking around with mouse, but Enable mouse to click and move in environment
          ;;;[1 1 1] Set Var "DisableInputAtStartInBP" to TRUE and "EnableMouseButton" to FALSE and "DisableWASDEnableMouseClickOnly" to TRUE to:
          ;;;
          ;;; Enable Mouse movement, but disable Player movement with WASD
          (Variables|Default|SetDisableWASDEnableMouseClickOnly false)
          (Input|SetIgnoreMoveInput (Game|GetPlayerController 0) (Variables|Default|GetDisableWASDEnableMouseClickOnly)))
        (:then_1
          ;;;[1 1 1] Set Var "DisableInputAtStartInBP" to TRUE and "EnableMouseButton" to FALSE and "DisableMouseLookEnableMouseClickOnly" to TRUE to:
          ;;;
          ;;; Enable Mouse movement, but disable Player looking around with mouse
          (Variables|Default|SetDisableMouseLookEnableMouseClickOnly true)
          (Input|SetIgnoreLookInput (Game|GetPlayerController 0) (Variables|Default|GetDisableMouseLookEnableMouseClickOnly))))
      (else
        ;;[1 1 1] Set Var "DisableInputAtStartInBP" to TRUE and "EnableMouseButton" to FALSE to:
        ;;
        ;; Disable ALL player input
        (Input|DisableInput (Game|GetPlayerCharacter 0) (Game|GetPlayerController 0))))
    (else
      ;;[1 1 1] Set Var "DisableInputAtStartInBP" to False to Enable ALL player input
      (Input|EnableInput (Game|GetPlayerCharacter 0) (Game|GetPlayerController 0)))))

(fn ConstructionScript)