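; Game instance that holds energy, anxiety, timer and other game state, and ends the game when energy or anxiety hits its limit.
; The game-over event shows the Game_Over widget and pauses play when energy is zero or anxiety is one, unless a dialogue widget is open.
; Init events wait briefly, cast to the player character and game mode, then push the stored energy, anxiety and timer values into them.
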(event Custom|GameInstanceINITVariables
  ;[1 1 1] Ref to player, enabling you to send info
  ;
  ; In PCCCharacter_Loc, this event is called at BeginPlay
  (Utilities|FlowControl|Delay 0.1)
  (bind _aspcccharacter_sprite_locations (Utilities|Casting|CastToPCCCharacterSprite_Locations (Game|GetPlayerCharacter 0)))
  (bind _output_get (Variables|Default|SetAs%20PCCCharacter%20Sprite%20Locations _aspcccharacter_sprite_locations))
  ;[1 1 1] Updates Player variables with GameInst variables.
  (Default|CallUpdateEnergyandAnxietyGameMode _output_get (Variables|Default|GetINT_Energy) (Variables|Default|GetINT_Anxiety)))

(event Custom|GameInstanceINTTImer
  (Utilities|FlowControl|Delay 0.1)
  (bind _asbp_game_mode_wasd_locations (Utilities|Casting|CastToBP_Game_Mode_WASD_Locations (Game|GetGameMode)))
  (bind _output_get (Variables|Default|SetAs%20BP%20Game%20Mode%20WASD%20Locations _asbp_game_mode_wasd_locations))
  (Default|UpdateTimerEvent _output_get (Variables|Default|GetINT_MInutes) (Variables|Default|GetINT_Seconds)))

(event Custom|GameEndFromAnxietyOrEnergyInGameInstance
  ;[1 1 1] Function in PCCCharacter_Locations & in NPC_WASD_AI_Controller. Checks if
  ; - Energy = 0 or Anxiety = 1
  ; - if dialogue widge open
  (if (or (== (Variables|Default|GetINT_Energy) 0.0) (== 1.0 (Variables|Default|GetINT_Anxiety)))
    (if (not (Variables|Default|GetINT_DialogueWidgetOpen))
      ;[1 1 1] Game over when timer = 0
      (bind _returnvalue (UserInterface|CreateWidget "/Game/Dialogue/BluePrints/MainMenu_Widget/Game_Over.Game_Over_C"))
      (UserInterface|Viewport|AddtoViewport _returnvalue 0)
      (Game|SetGamePaused true))))