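; Spline actor for the meditation mini-game that moves an "inner thought" actor along a spline path in an endless loop.
; BeginPlay picks a random actor from an array and sets the timeline play rate from a duration in seconds.
; The timeline lerps distance along the spline to set the actor's location and tangent-facing rotation, replaying when finished.
; The construction script snaps the selected actor to the spline's first point.
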(event Custom|Play_TimelineEvent
  (bind _spline (Variables|Default|GetSpline))
  (bind _spline_2 (Variables|Default|GetSpline))
  (bind _actorinnerthoughtselected (Variables|Default|GetActorInnerThoughtSelected))
  (bind _innerthoughttimelinefloattrack (Timeline|InnerThoughtTimeline PlayFromStart)
    (:Update
      ;[1 1 1] Moves Actor to new location along spline
      ;
      ; Make Variable type "Actor" object reference called "actor Innter Thought Selected" and connect to Target. This assigns an actor to this spline. Without specifying the target, this BP would assume a self reference.
      (Transformation|SetActorLocation _actorinnerthoughtselected (Spline|GetLocationatDistanceAlongSpline _spline (Math|Float|Lerp 0.0 (Spline|GetDistanceAlongSplineatSplinePoint _spline_2 (- (Spline|GetNumberOfSplinePoints _spline_2) 1)) _innerthoughttimelinefloattrack) "World") false false)
      ;[1 1 1] Makes actor face direction it's moving
      (Transformation|SetActorRotation _actorinnerthoughtselected (Math|Conversions|RotationFromXVector (Spline|GetTangentatDistanceAlongSpline _spline (Math|Float|Lerp 0.0 (Spline|GetDistanceAlongSplineatSplinePoint _spline_2 (- (Spline|GetNumberOfSplinePoints _spline_2) 1)) _innerthoughttimelinefloattrack) "World"))))
    (:Finished
      ;[1 1 1] Loops timeline after it finishes
      (CallFunction|PlayTimelineEvent))))

(event EventBeginPlay
  (bind _actorinnerthoughtselected_array (Variables|Default|GetActorInnerThoughtSelected_Array))
  ;[1 1 1] Set random actor to variable ActorInnerThoughSelected
  (Variables|Default|SetActorInnerThoughtSelected (Utilities|Array|Get(acopy) _actorinnerthoughtselected_array (Math|Random|RandomIntegerinRange 0 (Utilities|Array|LastIndex _actorinnerthoughtselected_array))))
  ;[1 1 1] Change
  (Development|PrintString "Hello")
  ;;[1 1 1] Adjusts Timeline length. Timeline length is at 1, so dividing 1/# adjust time
  (Components|Timeline|SetPlayRate (Variables|Default|GetInnerThoughtTimeline) (/ 1.0 (Variables|Default|GetInnerThoughtTimeLineLengthInSeconds)))
  (CallFunction|PlayTimelineEvent))

(event Collision|EventActorBeginOverlap
  (params (OtherActor :type Actor%20Object%20Reference)))

(event EventTick
  (params (DeltaSeconds :type Float%20%28single-precision%29)))

(fn ConstructionScript
  ;[1 1 1] When you select an actor to be on spline within the game editor, this script puts it at the begining of spline
  (Transformation|SetActorLocation (Variables|Default|GetActorInnerThoughtSelected) (Spline|GetLocationatSplinePoint (Variables|Default|GetSpline) 0 "World") false false))