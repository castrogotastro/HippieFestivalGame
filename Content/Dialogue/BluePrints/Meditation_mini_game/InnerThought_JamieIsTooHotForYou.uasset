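; Inner-thought trigger actor for the meditation mini-game that feeds worry messages to the player character.
; Each gated box overlap increments a counter, passing the first or second hardcoded thought about job and money to PCCCharacterSprite_Locations and calling InnerThoughtOverLap.
; The gate closes on overlap and reopens five seconds after overlap ends.
; Clicking the box runs a timeline that animates text opacity through a dynamic material instance created on BeginPlay.
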(event OnClicked(Box)
  (params (TouchedComponent :type Primitive%20Component%20Object%20Reference) (ButtonPressed :type Key%20Structure :default "None"))
  (bind _opacityfloattrack (Timeline|Timeline_0 Play)
    (:Update
      (Development|PrintString "ClickMe1")
      (Rendering|Material|SetScalarParameterValue (Variables|Default|GetDynmaticMaterialTextDefault) "Opacity" _opacityfloattrack :!class /Script/Engine.MaterialInstanceDynamic))))

(event OnComponentBeginOverlap(Box)
  (params (OverlappedComponent :type Primitive%20Component%20Object%20Reference) (OtherActor :type Actor%20Object%20Reference) (OtherComp :type Primitive%20Component%20Object%20Reference) (OtherBodyIndex :type Integer) (bFromSweep :type Boolean) (SweepResult :type Hit%20Result%20Structure%20%28by%20ref%29))
  (bind _as_pcccharacter_sprite_locations (Variables|Default|GetAs%20PCCCharacter%20Sprite%20Locations))
  (if (Variables|Default|GetOpenGate)
    (Variables|Default|SetOpenGate false)
    (Development|PrintString "BeginOverlap")
    (Variables|Default|SetInnerThoughtCount1 (+ (Variables|Default|GetInnerThoughtCount1) 1))
    (if (== (Variables|Default|GetInnerThoughtCount1) 1)
      (bind _output_get (Variables|Default|SetInnerThought1_message1 "You think about your job"))
      (Variables|/Game/Dialogue/BluePrints/Player_And_GameModes/PCCCharacterSprite_Locations.PCCCharacterSprite_Locations_C|SetInnerThoughtsToDisplay _as_pcccharacter_sprite_locations _output_get)
      (Development|PrintString "set string")
      (Default|InnerThoughtOverLap _as_pcccharacter_sprite_locations)
      (elif (== (Variables|Default|GetInnerThoughtCount1) 2)
        (bind _output_get_2 (Variables|Default|SetInnerThought1_message2 "Are you going to make enough money"))
        (Variables|/Game/Dialogue/BluePrints/Player_And_GameModes/PCCCharacterSprite_Locations.PCCCharacterSprite_Locations_C|SetInnerThoughtsToDisplay (Variables|Default|GetAs%20PCCCharacter%20Sprite%20Locations) _output_get_2)
        (Default|InnerThoughtOverLap _as_pcccharacter_sprite_locations)
        (else
          (Development|PrintString "false entry"))))))

(event OnComponentEndOverlap(Box)
  (params (OverlappedComponent :type Primitive%20Component%20Object%20Reference) (OtherActor :type Actor%20Object%20Reference) (OtherComp :type Primitive%20Component%20Object%20Reference) (OtherBodyIndex :type Integer))
  (Utilities|FlowControl|Delay 5.0)
  (Variables|Default|SetOpenGate true)
  (Development|PrintString "open fate")
  (Development|PrintString "OVERLAP ME"))

(event EventBeginPlay
  (bind _asgame_instance_wasd (Utilities|Casting|CastToGameInstance_WASD (Game|GetGameInstance)))
  (Variables|Default|SetAs%20Game%20Instance%20WASD _asgame_instance_wasd)
  (bind _aspcccharacter_sprite_locations (Utilities|Casting|CastToPCCCharacterSprite_Locations (Game|GetPlayerCharacter 0)))
  (Variables|Default|SetAs%20PCCCharacter%20Sprite%20Locations _aspcccharacter_sprite_locations)
  (bind _returnvalue (Rendering|Material|CreateDynamicMaterialInstance (Variables|Default|GetInnerThough_1) 0 "/Engine/EngineMaterials/DefaultTextMaterialTranslucentMODIFIED_Inst.DefaultTextMaterialTranslucentMODIFIED_Inst" "None" :!class /Script/Engine.PrimitiveComponent))
  (Variables|Default|SetDynmaticMaterialTextDefault _returnvalue))

(event Collision|EventActorBeginOverlap
  (params (OtherActor :type Actor%20Object%20Reference)))

(event EventTick
  (params (DeltaSeconds :type Float%20%28single-precision%29)))

(fn ConstructionScript)