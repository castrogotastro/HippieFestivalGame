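; BP_Dialogue_Trigger is a clickable actor that shows and hides a Widget_Dialogue box on screen.
; Clicking it removes the stored widget if one is open; otherwise it creates one, adds it to the viewport and copies VarTextDialogue into its DialogueText.
; A separate OnInteract event also creates and shows the widget, but without the open check or the text assignment.
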(event EventBeginPlay)

(event Collision|EventActorBeginOverlap
  (params (OtherActor :type Actor%20Object%20Reference)))

(event EventTick
  (params (DeltaSeconds :type Float%20%28single-precision%29)))

(event EventOnInteract
  (params (MouseInteractor :type Mouse%20Cursor%20Interactor%20Object%20Reference))
  (bind _returnvalue (UserInterface|CreateWidget "/Game/Dialogue/Widget/Widget_Dialogue.Widget_Dialogue_C" (Game|GetPlayerController 0)))
  (bind _output_get (Variables|Default|SetDialogueWidget _returnvalue))
  (UserInterface|Viewport|AddtoViewport _output_get 0))

(event MouseInput|EventActorOnClicked
  (params (ButtonPressed :type Key%20Structure :default "None"))
  ;[1 1 1] Open dialogue box when actor clicked
  ;;[1 1 1] Checks if dialogue box already open. If Actor clicked again, dialogue box closes
  (Utilities|IsValid (Variables|Default|GetDialogueWidget)
    (:Is%20Valid
      (Widget|RemovefromParent (Variables|Default|GetDialogueWidget))
      (Variables|Default|SetDialogueWidget 0))
    (:Is%20Not%20Valid
      (bind _returnvalue (UserInterface|CreateWidget "/Game/Dialogue/Widget/Widget_Dialogue.Widget_Dialogue_C" (Game|GetPlayerController 0)))
      (bind _output_get (Variables|Default|SetDialogueWidget _returnvalue))
      (UserInterface|Viewport|AddtoViewport _output_get 0)
      ;;[1 1 1] Link text var in widget to var text here
      (Variables|/Game/Dialogue/Widget/Widget_Dialogue.Widget_Dialogue_C|SetDialogueText (Variables|Default|GetDialogueWidget) (Variables|Default|GetVarTextDialogue)))))

(fn ConstructionScript)