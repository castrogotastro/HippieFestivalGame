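; Location sign actor that shows an area name near its trigger box and lets the player switch map signage to the camp material.
; Box overlap enables input and toggles the AreaName display, while leaving disables input after a short delay.
; Pressing E sets IconLocation to the camp location, then applies a dynamic SignCamp material, created at BeginPlay, to the static mesh on actors tagged LocationMapTag.
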(event OnComponentBeginOverlap(Box)
  (params (OverlappedComponent :type Primitive%20Component%20Object%20Reference) (OtherActor :type Actor%20Object%20Reference) (OtherComp :type Primitive%20Component%20Object%20Reference) (OtherBodyIndex :type Integer) (bFromSweep :type Boolean) (SweepResult :type Hit%20Result%20Structure%20%28by%20ref%29))
  (Input|EnableInput (Game|GetPlayerController 0))
  (Rendering|ToggleVisibility (Variables|Default|GetAreaName) false)
  (Utilities|FlowControl|Delay 2.0))

(event OnComponentEndOverlap(Box)
  (params (OverlappedComponent :type Primitive%20Component%20Object%20Reference) (OtherActor :type Actor%20Object%20Reference) (OtherComp :type Primitive%20Component%20Object%20Reference) (OtherBodyIndex :type Integer))
  (Utilities|FlowControl|Delay 1.0)
  (Input|DisableInput (Game|GetPlayerController 0))
  (Rendering|ToggleVisibility (Variables|Default|GetAreaName) false)
  (Utilities|FlowControl|Delay 2.0))

(event EventBeginPlay
  (bind _returnvalue (Rendering|Material|CreateDynamicMaterialInstance "/Game/IllustrationsCharacters/Icons/SignCamp_Mat.SignCamp_Mat" "None" "None" :!class /Script/Engine.KismetMaterialLibrary))
  (Variables|Default|SetBackground_Camp_Material _returnvalue))

(event Collision|EventActorBeginOverlap
  (params (OtherActor :type Actor%20Object%20Reference)))

(event EventTick
  (params (DeltaSeconds :type Float%20%28single-precision%29)))

(event Input|KeyboardEvents|E
  (params (Key :type Key%20Structure :default "None"))
  (:Pressed
    (Variables|Default|SetIconLocation (Variables|Default|GetLocation_camp))
    (Utilities|Casting|CastToPCCCharacterSprite (Game|Player|GetPlayerPawn 0))
    (Actor|GetAllActorsOfClass "/Script/Engine.Actor")
    (for _array_element 0
      (if (Actor|ActorHasTag "LocationMapTag")
        (for (_array_element_2 _array_index) (Utilities|Array|MakeArray (Actor|GetComponentbyClass _array_element "/Script/Engine.StaticMeshComponent"))
          (for _index (range 0 (- (Rendering|Material|GetNumMaterials _array_element_2) 1))
            (Rendering|Material|SetMaterial _array_element_2 _array_index (Variables|Default|GetBackground_Camp_Material))))))))

(fn ConstructionScript)