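; A location signpost actor that shows an area name and acts as a clickable travel point to the Campsite3 level.
; Box overlap enables actor input and toggles the name's visibility; leaving disables input and toggles it again after a short delay.
; Clicking the box fades the camera out, checks for the PCCCharacterSprite player, then opens the level and requests a fade-in.
; Map icon recolouring and a HUD fade remain as unconnected experiments.
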(event OnComponentBeginOverlap(Box)
  (params (OverlappedComponent :type Primitive%20Component%20Object%20Reference) (OtherActor :type Actor%20Object%20Reference) (OtherComp :type Primitive%20Component%20Object%20Reference) (OtherBodyIndex :type Integer) (bFromSweep :type Boolean) (SweepResult :type Hit%20Result%20Structure%20%28by%20ref%29))
  (Input|EnableInput (Game|GetPlayerController 0))
  (Rendering|ToggleVisibility (Variables|Default|GetAreaName) false)
  (Utilities|FlowControl|Delay 2.0))

(event OnClicked(Box)
  (params (TouchedComponent :type Primitive%20Component%20Object%20Reference) (ButtonPressed :type Key%20Structure))
  (CameraFades|StartCameraFade :self (Game|GetPlayerCameraManager 0) :ToAlpha 1.0 :Duration 3.0 :bShouldFadeAudio true :bHoldWhenFinished true)
  (Utilities|FlowControl|Delay 4.0)
  (Utilities|Casting|CastToPCCCharacterSprite (Game|GetPlayerCharacter 0))
  (Game|OpenLevel(byObjectReference) "/Game/LVL/Maps/Campsite3.Campsite3")
  (Utilities|FlowControl|Delay 1.0)
  (CameraFades|StartCameraFade :self (Game|GetPlayerCameraManager 0) :FromAlpha 1.0 :Duration 3.0))

(event OnComponentEndOverlap(Box)
  (params (OverlappedComponent :type Primitive%20Component%20Object%20Reference) (OtherActor :type Actor%20Object%20Reference) (OtherComp :type Primitive%20Component%20Object%20Reference) (OtherBodyIndex :type Integer))
  (Utilities|FlowControl|Delay 1.0)
  (Input|DisableInput (Game|GetPlayerController 0))
  (Rendering|ToggleVisibility (Variables|Default|GetAreaName) false)
  (Utilities|FlowControl|Delay 2.0))

(event EventBeginPlay
  (bind _returnvalue (Rendering|Material|CreateDynamicMaterialInstance "/Game/LVL/IllustrationsCharacters/Icons/SignCamp_Mat.SignCamp_Mat" "None" "None" :!class /Script/Engine.KismetMaterialLibrary))
  (Variables|Default|SetBackground_Camp_Material _returnvalue))

(event Collision|EventActorBeginOverlap
  (params (OtherActor :type Actor%20Object%20Reference)))

(event EventTick
  (params (DeltaSeconds :type Float%20%28single-precision%29)))

(fn ConstructionScript)